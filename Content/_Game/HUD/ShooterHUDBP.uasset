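; HUD Blueprint for the shooter that draws a dynamic four-piece crosshair slightly above screen centre.
; It caches the player pawn as a ShooterCharacterBP on BeginPlay, retrying the cast during DrawHUD if the reference is invalid.
; Each DrawHUD call reads the character's crosshair spread multiplier, scales it by a maximum spread, and offsets the top, bottom, left and right textures outward from the crosshair centre.
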(event EventDrawHUD
  (params (SizeX :type Integer) (SizeY :type Integer))
  ;[1 1 1] Set screen centre and crosshair location
  (Variables|Default|SetScreen%20Centre (Math|Vector2D|MakeVector2D (Math|Conversions|ToFloat(Integer) (/ SizeX 2)) (Math|Conversions|ToFloat(Integer) (/ SizeY 2))))
  (Variables|Default|SetCrosshairLocation (Math|Vector2D|MakeVector2D (.X (Math|Vector2D|BreakVector2D (Variables|Default|GetScreen%20Centre))) (- (.Y (Math|Vector2D|BreakVector2D (Variables|Default|GetScreen%20Centre))) 5e+01)))
  ;[1 1 1] Make sure ref to Shooter Character is valid
  (Utilities|IsValid (Variables|Default|GetShooterCharacter)
    (:Is%20Valid
      _)
    (:Is%20Not%20Valid
      (bind _asshooter_character_bp (Utilities|Casting|CastToShooterCharacterBP (Game|Player|GetPlayerPawn 0)))
      (Variables|Default|SetShooterCharacter _asshooter_character_bp)))
  ;[1 1 1] Get crosshair spread multiplier
  (Variables|Default|SetCrosshairSpreadMultiplier (Class|ShooterCharacter|GetCrosshairSpreadMultiplier (Variables|Default|GetShooterCharacter)))
  ;[1 1 1] Centre of crosshair location
  (Variables|Default|SetCrosshairBaseCentre (Math|Vector2D|MakeVector2D (- (.X (Math|Vector2D|BreakVector2D (Variables|Default|GetCrosshairLocation))) (Variables|Default|GetCrossHairHalfWidth)) (- (.Y (Math|Vector2D|BreakVector2D (Variables|Default|GetCrosshairLocation))) (Variables|Default|GetCrossHairHalfHeight))))
  (Utilities|FlowControl|Sequence
    (:then_0
      (Canvas|DrawTexture "/Game/_Game/Assets/Textures/Crosshairs/Crosshair_Quad_9_Bottom.Crosshair_Quad_9_Bottom" (.X (Math|Vector2D|BreakVector2D (Variables|Default|GetCrosshairBaseCentre))) (+ (.Y (Math|Vector2D|BreakVector2D (Variables|Default|GetCrosshairBaseCentre))) (* (Variables|Default|GetCrosshairSpreadMultiplier) (Variables|Default|GetCrosshairSpreadMax))) 64.0 64.0 0.0 0.0 1.0 1.0 "(R=1.000000,G=1.000000,B=1.000000,A=1.000000)")
      (Canvas|DrawTexture "/Game/_Game/Assets/Textures/Crosshairs/Crosshair_Quad_9_Top.Crosshair_Quad_9_Top" (.X (Math|Vector2D|BreakVector2D (Variables|Default|GetCrosshairBaseCentre))) (- (.Y (Math|Vector2D|BreakVector2D (Variables|Default|GetCrosshairBaseCentre))) (* (Variables|Default|GetCrosshairSpreadMultiplier) (Variables|Default|GetCrosshairSpreadMax))) 64.0 64.0 0.0 0.0 1.0 1.0 "(R=1.000000,G=1.000000,B=1.000000,A=1.000000)"))
    (:then_1
      (Canvas|DrawTexture "/Game/_Game/Assets/Textures/Crosshairs/Crosshair_Quad_9_Left.Crosshair_Quad_9_Left" (- (.X (Math|Vector2D|BreakVector2D (Variables|Default|GetCrosshairBaseCentre))) (* (Variables|Default|GetCrosshairSpreadMultiplier) (Variables|Default|GetCrosshairSpreadMax))) (.Y (Math|Vector2D|BreakVector2D (Variables|Default|GetCrosshairBaseCentre))) 64.0 64.0 0.0 0.0 1.0 1.0 "(R=1.000000,G=1.000000,B=1.000000,A=1.000000)")
      (Canvas|DrawTexture "/Game/_Game/Assets/Textures/Crosshairs/Crosshair_Quad_9_Right.Crosshair_Quad_9_Right" (+ (.X (Math|Vector2D|BreakVector2D (Variables|Default|GetCrosshairBaseCentre))) (* (Variables|Default|GetCrosshairSpreadMultiplier) (Variables|Default|GetCrosshairSpreadMax))) (.Y (Math|Vector2D|BreakVector2D (Variables|Default|GetCrosshairBaseCentre))) 64.0 64.0 0.0 0.0 1.0 1.0 "(R=1.000000,G=1.000000,B=1.000000,A=1.000000)"))))

(event EventBeginPlay
  ;[1 1 1] Get a reference to the Shooter Character
  (Utilities|IsValid (Variables|Default|GetShooterCharacter)
    (:Is%20Not%20Valid
      (bind _asshooter_character_bp (Utilities|Casting|CastToShooterCharacterBP (Game|Player|GetPlayerPawn 0)))
      (Variables|Default|SetShooterCharacter _asshooter_character_bp))))

(fn ConstructionScript)